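; BP_EnemyBiped is an enemy biped Blueprint that gives visual feedback when its health changes.
; On each attribute component health change, it writes the current health percent to a scalar parameter on the mesh materials.
; On damage it also stamps the game time into a time-to-hit material parameter and spawns a damage pop-up widget attached to itself.
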(event `self.EnemyAttributeComp.OnHealthChanged`
  (params (InstigatorActor :type "Actor Object Reference") (OwningComp :type "CAttributeComponentBase Object Reference") (Delta :type "Float (single-precision)") (NewHealth :type "Float (single-precision)"))
  (bind _mesh (`self.Mesh`))
  (bind _returnvalue (`self.GetHealthPercent`))
  (`MeshComponent.SetScalarParameterValueOnMaterials` _mesh "HealthPercent" _returnvalue)
  (if (< Delta 0.0)
    (`MeshComponent.SetScalarParameterValueOnMaterials` _mesh (`self.TimeToHitParamName`) (`KismetSystemLibrary.GetGameTimeInSeconds`))
    (bind _returnvalue_2 (`|CreateWidget` "/Game/Nyx/UI/W_DamagePopUp.W_DamagePopUp_C" (`GameplayStatics.GetPlayerController` 0) self))
    (`UserWidget.AddToViewport` _returnvalue_2 0)))

(fn `UserConstructionScript`)