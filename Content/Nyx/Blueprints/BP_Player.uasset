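; Player pawn for a physics-driven, thrust-based flying craft with crosshair and health widgets.
; Tick eases velocity toward forward speed, damps spin and yaws the mesh toward the spring arm, which camera input rotates.
; Looping timers step thrust and repeat projectile fire while inputs are held.
; Direct roll, pitch and yaw inputs are empty; their old handlers and thrust-scaled gravity are disconnected.
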(event `InputAxis|RollLeft`
  (params (AxisValue :type "Float (single-precision)"))
  ;[1 1 1] Movement
)

(event `InputAxis|RollRight`
  (params (AxisValue :type "Float (single-precision)"))
  ;[1 1 1] Movement
)

(event `InputAxis|YawRight`
  (params (AxisValue :type "Float (single-precision)"))
  ;[1 1 1] Movement
)

(event `InputAxis|YawLeft`
  (params (AxisValue :type "Float (single-precision)"))
  ;[1 1 1] Movement
)

(event `InputAxis|PitchUp`
  (params (AxisValue :type "Float (single-precision)"))
  ;[1 1 1] Movement
)

(event `InputAxis|PitchDown`
  (params (AxisValue :type "Float (single-precision)"))
  ;[1 1 1] Movement
)

(event `InputAction|IncreaseThrust`
  (params (Key :type "Key Structure"))
  ;[1 1 1] Adjust Thrust
  (:`Pressed`
    (set `self.bIncreasingThrust` true)
    (bind _returnvalue (`self.GetThrust` :!label _label))
    (`KismetSystemLibrary.PrintString` (`KismetStringLibrary.Concat_StrStr` "Thrust: " (`KismetStringLibrary.Conv_DoubleToString` _returnvalue))))
  (:`Released`
    (set `self.bIncreasingThrust` false)
    (goto _label)))

(event `InputAction|DecreaseThrust`
  (params (Key :type "Key Structure"))
  ;[1 1 1] Adjust Thrust
  (:`Pressed`
    (set `self.bDecreasingThrust` true)
    (goto _label))
  (:`Released`
    (set `self.bDecreasingThrust` false)
    (goto _label)))

(event `self.ReceiveBeginPlay`
  (`parent.ReceiveBeginPlay`)
  (bind _returnvalue (`|CreateWidget` "/Game/Nyx/UI/W_Crosshair.W_Crosshair_C"))
  (`UserWidget.AddToViewport` _returnvalue 0)
  (bind _returnvalue_2 (`|CreateWidget` "/Game/Nyx/UI/W_PlayerHealth.W_PlayerHealth_C"))
  (`UserWidget.AddToViewport` _returnvalue_2 0)
  ;[1 1 1] Checks input for thrust adjustment
  (`KismetSystemLibrary.K2_SetTimer` null "AdjustThrust" 0.05 true))

(event `self.ReceiveTick`
  (params (DeltaSeconds :type "Float (single-precision)"))
  (bind _meshcomp (`self.MeshComp`))
  (bind _meshcomp_2 (`self.MeshComp`))
  (bind _meshcomp_3 (`self.MeshComp`))
  (bind _yaw (.yaw (`SceneComponent.K2_GetComponentRotation` (`self.MeshComp`))))
  (bind _yaw_2 (.yaw (`SpringArmComponent.GetTargetRotation` (`self.SpringArmComp`))))
  (bind _returnvalue (- _yaw_2 _yaw))
  (`parent.ReceiveTick` 0.0)
  ;[1 1 1] Friction against angular velocity
  (`PrimitiveComponent.AddTorqueInDegrees` _meshcomp_2 (* (`KismetMathLibrary.NegateVector` (`PrimitiveComponent.GetPhysicsAngularVelocityInDegrees` _meshcomp_2 "None")) (`KismetMathLibrary.SelectFloat` 0.9 0.0 true)) "None" true)
  ;[1 1 1] Forward movement
  (bind _returnvalue_2 (`PrimitiveComponent.GetPhysicsLinearVelocity` _meshcomp_3 "None"))
  (bind _returnvalue_3 (`self.GetSpeed`))
  (`PrimitiveComponent.SetAllPhysicsLinearVelocity` _meshcomp_3 (`KismetMathLibrary.VLerp` _returnvalue_2 (* _returnvalue_3 (`self.GetActorForwardVector`)) 0.01) false)
  (if (`KismetMathLibrary.NearlyEqual_FloatFloat` _yaw_2 _yaw 1.0)
    (`PrimitiveComponent.SetAllPhysicsAngularVelocityInDegrees` _meshcomp (* (`PrimitiveComponent.GetPhysicsAngularVelocityInDegrees` _meshcomp "None") 0.8) false)
    (else
      (`self.HandleRotationInput` (/ _returnvalue (`KismetMathLibrary.Abs` _returnvalue)) (`SceneComponent.GetUpVector` (`self.MeshComp`)) 0.1))))

(event `InputAction|AttackPrimary`
  (params (Key :type "Key Structure"))
  (:`Pressed`
    (`self.FireProjectile`)
    (`KismetSystemLibrary.K2_SetTimer` null "FireProjectile" 0.5 true))
  (:`Released`
    (`KismetSystemLibrary.K2_ClearTimer` null "FireProjectile")))

(event `InputAxis|CameraPitch`
  (params (AxisValue :type "Float (single-precision)"))
  ;[1 1 1] Rotate camera
  (`SceneComponent.K2_AddRelativeRotation` (`self.SpringArmComp`) (`KismetMathLibrary.MakeRotator` 0.0 (* (/ AxisValue (`KismetMathLibrary.Abs` AxisValue)) (`self.CameraRotationSpeed`))) false false))

(event `InputAxis|CameraYaw`
  (params (AxisValue :type "Float (single-precision)"))
  ;[1 1 1] Rotate camera
  (`SceneComponent.K2_AddRelativeRotation` (`self.SpringArmComp`) (`KismetMathLibrary.MakeRotator` 0.0 0.0 (* (/ AxisValue (`KismetMathLibrary.Abs` AxisValue)) (`self.CameraRotationSpeed`))) false false))

(event `self.AttributeComp.OnPlayerHealthChangedDelegate`
  (params (InstigatorActor :type "Actor Object Reference") (OwningComp :type "CAttributeComponent Object Reference") (Delta :type "Float (single-precision)") (NewHealth :type "Float (single-precision)"))
  (`KismetSystemLibrary.PrintString` (`KismetStringLibrary.Conv_DoubleToString` NewHealth) true true (struct :`R` 0.461158 :`B` 1.0 :`A` 1.0)))

(fn `AdjustThrust`
  (if (`self.bIncreasingThrust`)
    (`self.IncrementThrust`)
    (elif (`self.bDecreasingThrust`)
      (`self.DecrementThrust`))))

(fn `CalculateGravityInfluence`
  (returns (Out :type "Float (double-precision)"))
  (bind _returnvalue (`self.GetThrust`))
  (return (* (- 1.0 (/ _returnvalue 100.0)) (`self.GravityConstant`))))

(fn `FireProjectile`
  (`self.SpawnProjectile` "/Game/Nyx/Blueprints/BP_Projectile.BP_Projectile_C"))

(fn `UserConstructionScript`)