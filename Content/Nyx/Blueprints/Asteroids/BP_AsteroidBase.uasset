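; Base asteroid Blueprint that adds visual damage feedback to the asteroid's Sphere mesh when its health changes.
; OnHealthChanged routes to a handler that triggers a hit flash and color update, then calls the parent implementation.
; Both effects set material scalars: TimeToHit stamps the game time of the hit, and HealthPercent reflects the AttributeComp's health.
; A PrintAttributes debug helper prints power, health and size attributes.
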(event `self.OnHealthChanged`
  (params (InstigatorActor :type "Actor Object Reference") (OwningComp :type "CAsteroidAttributeComponent Object Reference") (Delta :type "Float (single-precision)") (NewHealth :type "Float (single-precision)"))
  (`self.HealthChangedHandler` InstigatorActor OwningComp Delta NewHealth))

(fn `ExecuteHitFlash`
  (`MeshComponent.SetScalarParameterValueOnMaterials` (`self.Sphere`) "TimeToHit" (`KismetSystemLibrary.GetGameTimeInSeconds`)))

(fn `HealthChangedHandler`
  (params (InstigatorActor :type "Actor Object Reference") (OwningComp :type "CAsteroidAttributeComponent Object Reference") (Delta :type "Float (single-precision)") (NewHealth :type "Float (single-precision)"))
  (`self.ExecuteHitFlash`)
  (`self.UpdateColor`)
  (`parent.OnHealthChanged` InstigatorActor OwningComp Delta NewHealth))

(fn `PrintAttributes`
  (bind _attributecomp (`self.AttributeComp`))
  (`KismetSystemLibrary.PrintString` (`KismetStringLibrary.Concat_StrStr` (`KismetStringLibrary.Conv_DoubleToString` (`CAsteroidAttributeComponent.BasePower` _attributecomp)) "  --  " (`KismetStringLibrary.Conv_DoubleToString` (`CAsteroidAttributeComponent.Power` _attributecomp))) true true (struct :`G` 1.0 :`B` 0.25 :`A` 1.0) 20.0)
  (`KismetSystemLibrary.PrintString` (`KismetStringLibrary.Concat_StrStr` (`KismetStringLibrary.Conv_DoubleToString` (`CAsteroidAttributeComponent.BaseHealth` _attributecomp)) "  --  " (`KismetStringLibrary.Conv_DoubleToString` (`CAsteroidAttributeComponent.Health` _attributecomp))) true true (struct :`G` 1.0 :`B` 0.094607 :`A` 1.0) 20.0)
  (`KismetSystemLibrary.PrintString` (`KismetStringLibrary.Concat_StrStr` (`|GetEnumeratorNameAsString` (`CAsteroidAttributeComponent.Size` _attributecomp)) "  --  " (`KismetStringLibrary.Conv_DoubleToString` (`CAsteroidAttributeComponent.SizeMultiplier` _attributecomp))) true true (struct :`G` 1.0 :`B` 0.223963 :`A` 1.0) 20.0))

(fn `UpdateColor`
  (`MeshComponent.SetScalarParameterValueOnMaterials` (`self.Sphere`) "HealthPercent" (`CAsteroidAttributeComponent.GetHealthPercent` (`self.AttributeComp`))))

(fn `UserConstructionScript`)