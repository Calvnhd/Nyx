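; BP_BallSpawner is an asteroid spawner that releases asteroids from the location of its Torus component.
; It overrides SpawnOnce, calling the parent to spawn the asteroid, then firing its RadialForce impulse.
; It then applies AttributeModifier to the new asteroid's CAsteroidAttributeComponent and sets how many child asteroids it will spawn.
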(fn `GetSpawnLocation`
  (returns (ReturnValue :type "Vector Structure"))
  (return (`SceneComponent.K2_GetComponentLocation` (`self.Torus`))))

(fn `SpawnOnce`
  (returns (ReturnValue :type "CAsteroidBase Object Reference"))
  (locals (AsteroidSpawned :type "CAsteroidBase Object Reference"))
  (bind _returnvalue (`parent.SpawnOnce`))
  (set `local.AsteroidSpawned` _returnvalue)
  (`RadialForceComponent.FireImpulse` (`self.RadialForce`))
  (bind _returnvalue_2 (`CAttributeComponentBase.GetAttributes` (`local.AsteroidSpawned`)))
  (bind _ascasteroid_attribute_component (cast `CAsteroidAttributeComponent` _returnvalue_2))
  (`CAsteroidAttributeComponent.ModifyAttributes` _ascasteroid_attribute_component (`self.AttributeModifier`))
  (`CAsteroidAttributeComponent.SetNumberOfAsteroidsToSpawn` _ascasteroid_attribute_component (`self.NumberOfAsteroidChildrenToSpawn`))
  (return (`local.AsteroidSpawned`)))

(fn `UserConstructionScript`)