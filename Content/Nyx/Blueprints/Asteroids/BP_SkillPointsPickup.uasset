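; BP_SkillPointsPickup is an asteroid-game object that can be suctioned, armed and detonated; despite its name, it contains no skill point logic.
; Hitting an actor with an asteroid attribute component applies collision damage to that actor.
; StopSuction and Arm extend parent behavior by activating held and thrown effects respectively.
; Detonate runs a handler for blast damage and stun, a radial impulse and explosion particles, then calls the parent.
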(event `self.ReceiveTick`
  (params (DeltaSeconds :type "Float (single-precision)"))
  (`parent.ReceiveTick` DeltaSeconds))

(event `self.MeshComp.OnComponentHit`
  (params (HitComponent :type "PrimitiveComponent Object Reference") (OtherActor :type "Actor Object Reference") (OtherComp :type "PrimitiveComponent Object Reference") (NormalImpulse :type "Vector Structure") (Hit :type "HitResult Structure (by ref)"))
  (bind _returnvalue (`CAttributeComponentBase.GetAttributes` OtherActor))
  (bind _ascasteroid_attribute_component (cast `CAsteroidAttributeComponent` _returnvalue))
  (`CAttributeComponentBase.ApplyHealthChange` _ascasteroid_attribute_component null (* (`self.CollisionDamageAmount`) -1.0)))

(event `CBombInterface.Detonate`
  (`self.DetonateHandler`)
  (`parent.Detonate`))

(event `CPickupInterface.StopSuction`
  (params (InstigatorPawn :type "Pawn Object Reference"))
  (`parent.StopSuction` null)
  (`ActorComponent.Activate` (`self.HeldFX`) false))

(event `CBombInterface.Arm`
  (`parent.Arm`)
  (`ActorComponent.Activate` (`self.ThrownFX`) false))

(fn `DetonateHandler`
  (`self.BlastDamageAndStun`)
  (`RadialForceComponent.FireImpulse` (`self.RadialForce`))
  (`GameplayStatics.SpawnEmitterAtLocation` "/Game/Realistic_Starter_VFX_Pack_Vol2/Particles/Explosion/P_Explosion_Big_A.P_Explosion_Big_A" (`self.K2_GetActorLocation`)))

(fn `UserConstructionScript`)